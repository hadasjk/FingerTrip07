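; BP_Mobile is a decorative actor, apparently a hanging mobile, that spins its mesh components continuously.
; Each Tick rotates Torus002 in local yaw by RotateSpeed and Plane008, Plane009 and Plane010 by SubRotate, both scaled by delta time for frame-rate independence.
; Plane011 also receives a rotation call, but with zero yaw, so that call adds no rotation.
; BeginPlay, overlap and the construction script are empty.
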(event EventBeginPlay)

(event Collision|EventActorBeginOverlap
  (params (OtherActor :type Actor%20Object%20Reference)))

(event EventTick
  (params (DeltaSeconds :type Float%20%28single-precision%29))
  (bind _subrotate (Variables|Default|GetSubRotate))
  (bind _returnvalue (* DeltaSeconds _subrotate))
  (Transformation|AddLocalRotation (Variables|Default|GetTorus_002) (Math|Rotator|MakeRotator 0.0 0.0 (* DeltaSeconds (Variables|Default|GetRotateSpeed))) false false)
  (Transformation|AddLocalRotation (Variables|Default|GetPlane_009) (Math|Rotator|MakeRotator 0.0 0.0 _returnvalue) false false)
  (Transformation|AddLocalRotation (Variables|Default|GetPlane_008) (Math|Rotator|MakeRotator 0.0 0.0 _returnvalue) false false)
  (Transformation|AddLocalRotation (Variables|Default|GetPlane_010) (Math|Rotator|MakeRotator 0.0 0.0 _returnvalue) false false)
  (Transformation|AddLocalRotation (Variables|Default|GetPlane_011) (Math|Rotator|MakeRotator 0.0 0.0 0.0) false false))

(fn ConstructionScript)