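; BP_SpecialCoin is a collectible special coin that the BP_Finger player picks up in FingerTrip.
; When BP_Finger overlaps its sphere, it plays a coin sound, adds one to that finger's special coin score and destroys itself.
; Tick spins the coin around its roll axis at the Rotation speed.
; A Niagara pickup effect spawn exists but is not connected, so it never runs.
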(event OnComponentBeginOverlap(Sphere)
  (params (OverlappedComponent :type Primitive%20Component%20Object%20Reference) (OtherActor :type Actor%20Object%20Reference) (OtherComp :type Primitive%20Component%20Object%20Reference) (OtherBodyIndex :type Integer) (bFromSweep :type Boolean) (SweepResult :type Hit%20Result%20Structure%20%28by%20ref%29))
  (bind _asbp_finger (Utilities|Casting|CastToBP_Finger OtherActor))
  (Audio|PlaySoundatLocation "/Game/FingerTrip/Sounds/coin.coin" (Transformation|GetActorLocation) "0, 0, 0" 1.0 1.0 0.0 0 0 0 0)
  (Class|FingerCharacter|AddSpecialCoinScore _asbp_finger 1)
  (Actor|DestroyActor))

(event Collision|EventActorBeginOverlap
  (params (OtherActor :type Actor%20Object%20Reference)))

(event EventTick
  (params (DeltaSeconds :type Float%20%28single-precision%29))
  (Transformation|AddActorLocalRotation (Math|Rotator|MakeRotator (* DeltaSeconds (Variables|Default|GetRotation)) 0.0 0.0) false false))

(fn ConstructionScript)