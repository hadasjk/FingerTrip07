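; BP_Finger is a jumping character, likely the FingerTrip player, that restores its spawn position from a loaded save and plays a sound on jump.
; On BeginPlay it teleports to the game instance's target location if a save is loading, clears that flag, then starts a five-second, non-looping autosave timer.
; The autosave writes a new save object with total play time and level name, but no location, to a fixed slot.
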(event Custom|AutoSaveEvent
  (bind _returnvalue (SaveGame|CreateSaveGameObject "/Game/MH/Blueprint/BP_FingerTripSave.BP_FingerTripSave_C"))
  (bind _asbp_my_game_instance (Utilities|Casting|CastToBP_MyGameInstance (Game|GetGameInstance)))
  (Variables|/Game/MH/Blueprint/BP_FingerTripSave.BP_FingerTripSave_C|SetSavedPlayTime _returnvalue (Variables|/Game/FingerTrip/Blueprint/BP_MyGameInstance.BP_MyGameInstance_C|GetTotalPlayTime _asbp_my_game_instance))
  (bind _returnvalue_2 (Game|GetCurrentLevelName true))
  (Variables|/Game/MH/Blueprint/BP_FingerTripSave.BP_FingerTripSave_C|SetSavedLevelName _returnvalue (Utilities|String|StringToName _returnvalue_2))
  (SaveGame|SaveGametoSlot _returnvalue "Save1"))

(event EventBeginPlay
  (bind _asbp_my_game_instance (Utilities|Casting|CastToBP_MyGameInstance (Game|GetGameInstance)))
  (if (Variables|/Game/FingerTrip/Blueprint/BP_MyGameInstance.BP_MyGameInstance_C|GetbIsLoadingSave _asbp_my_game_instance)
    (Transformation|SetActorLocation (Variables|/Game/FingerTrip/Blueprint/BP_MyGameInstance.BP_MyGameInstance_C|GetTargetSpawnLocation _asbp_my_game_instance) false false)
    (Variables|/Game/FingerTrip/Blueprint/BP_MyGameInstance.BP_MyGameInstance_C|SetbIsLoadingSave _asbp_my_game_instance false))
  (Utilities|Time|SetTimerbyEvent (delegate Custom|AutoSaveEvent) 5.0))

(event Collision|EventActorBeginOverlap
  (params (OtherActor :type Actor%20Object%20Reference)))

(event EventTick
  (params (DeltaSeconds :type Float%20%28single-precision%29)))

(event EventOnJumped
  (Audio|PlaySound2D "/Game/FingerTrip/Sounds/JumpSound.JumpSound" 1.5 1.0 0.0 0 0))

(fn ConstructionScript)