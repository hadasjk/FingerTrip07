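; BP_MyGameInstance is the FingerTrip game instance, holding total play time and state for restoring a saved game.
; AddPlayTime adds a given delta to the running play time total.
; Unconnected load logic reads slot Save1 as BP_FingerTripSave, copies play time and spawn location, flags IsLoadingSave and opens the saved level.
; The Init event is empty, so nothing here runs that load.
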(event EventInit)

(fn AddPlayTime
  (params (DeltaTime :type Float%20%28double-precision%29))
  (Variables|Default|SetTotalPlayTime (+ DeltaTime (Variables|Default|GetTotalPlayTime))))