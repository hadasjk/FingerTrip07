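; BP_LevelManager is a level manager that shows end-of-level and settings UI.
; On BeginPlay it caches the player's FingerCharacter and starts a looping timer that polls its level-cleared and game-ended flags.
; Either flag opens WBP_Result with the cursor, guarded by DoOnce.
; ToggleMenu opens WBP_GameSetting, pauses the game and shows the cursor.
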(event Custom|ShowUI
  (bind _as_finger_character (Variables|Default|GetAs%20Finger%20Character))
  (if (Variables|/Script/FingerTrip.FingerCharacter|GetbIsLevelCleared _as_finger_character)
    (Utilities|FlowControl|DoOnce false
      (:Completed
        (bind _returnvalue (UserInterface|CreateWidget "/Game/FingerTrip/UI/WBP_Result.WBP_Result_C"))
        (bind _output_get (Variables|Default|SetClearWidget _returnvalue))
        (UserInterface|Viewport|AddtoViewport _output_get 0)
        (Variables|/Script/Engine.PlayerController|SetbShowMouseCursor (Game|GetPlayerController 0) true)))
    (elif (Variables|/Script/FingerTrip.FingerCharacter|GetbHasGameEnded _as_finger_character)
      (Utilities|FlowControl|DoOnce false
        (:Completed
          (bind _returnvalue_2 (UserInterface|CreateWidget "/Game/FingerTrip/UI/WBP_Result.WBP_Result_C"))
          (bind _output_get_2 (Variables|Default|SetClearWidget _returnvalue_2))
          (UserInterface|Viewport|AddtoViewport _output_get_2 0)
          (Variables|/Script/Engine.PlayerController|SetbShowMouseCursor (Game|GetPlayerController 0) true))))))

(event EventBeginPlay
  (Input|EnableInput (Game|GetPlayerController 0))
  (bind _asfinger_character (Utilities|Casting|CastToFingerCharacter (Game|GetPlayerCharacter 0)))
  (Variables|Default|SetAs%20Finger%20Character _asfinger_character)
  (Utilities|Time|SetTimerbyEvent (delegate Custom|ShowUI) 1.0 true))

(event Input|ActionEvents|InputActionToggleMenu
  (params (Key :type Key%20Structure :default "None"))
  (:Pressed
    (bind _returnvalue (UserInterface|CreateWidget "/Game/FingerTrip/UI/WBP_GameSetting.WBP_GameSetting_C"))
    (bind _output_get (Variables|Default|Setsettingwidget _returnvalue))
    (UserInterface|Viewport|AddtoViewport _output_get 0)
    (Game|SetGamePaused true)
    (Variables|/Script/Engine.PlayerController|SetbShowMouseCursor (Game|GetPlayerController 0) true)))

(fn ConstructionScript)