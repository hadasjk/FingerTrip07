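; BP_Arrive_MH is an ordered goal marker that BP_Finger_Tutorial must reach, forming a chain of waypoints.
; On BeginPlay it hides its spotlight and cylinder, and only the marker with the first GoalOrder activates itself, making both visible.
; When the finger begins overlapping an active marker's Box, it searches all BP_Arrive_MH actors, activates those with the next GoalOrder, then destroys itself.
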(event OnComponentBeginOverlap(Box)
  (params (OverlappedComponent :type Primitive%20Component%20Object%20Reference) (OtherActor :type Actor%20Object%20Reference) (OtherComp :type Primitive%20Component%20Object%20Reference) (OtherBodyIndex :type Integer) (bFromSweep :type Boolean) (SweepResult :type Hit%20Result%20Structure%20%28by%20ref%29))
  (if (Variables|Default|GetIsActive)
    (Utilities|Casting|CastToBP_Finger_Tutorial OtherActor)
    (bind _outactors (Actor|GetAllActorsOfClass "BP_Arrive_MH_C"))
    (for _array_element _outactors
      (if (== (Variables|BP_Arrive_MH_C|GetGoalOrder _array_element) (+ (Variables|Default|GetGoalOrder) 1))
        (CallFunction|ActivateTrigger _array_element)))
    (Actor|DestroyActor)))

(event Custom|ActivateTrigger
  (Variables|Default|SetIsActive true)
  (Rendering|SetVisibility (Variables|Default|GetCylinder) true false))

(event EventBeginPlay
  (Rendering|SetVisibility (Variables|Default|GetSpotLight) false false)
  (if (== (Variables|Default|GetGoalOrder) 1)
    (CallFunction|ActivateTrigger)))

(event Collision|EventActorBeginOverlap
  (params (OtherActor :type Actor%20Object%20Reference)))

(event EventTick
  (params (DeltaSeconds :type Float%20%28single-precision%29)))

(fn ConstructionScript)