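; BP_Rocket is a rocket actor that launches when a BP_Finger overlaps its Trigger, shaking the camera and activating its NS effect.
; Two timelines, timed by variables, lerp the actor from its start to MidLocation, then after a pause onward by WallDistance.
; After a cooldown it snaps back to its start location and deactivates the effect.
; An unconnected node for attaching the finger to the rocket never runs.
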(event OnComponentBeginOverlap(Trigger)
  (params (OverlappedComponent :type Primitive%20Component%20Object%20Reference) (OtherActor :type Actor%20Object%20Reference) (OtherComp :type Primitive%20Component%20Object%20Reference) (OtherBodyIndex :type Integer) (bFromSweep :type Boolean) (SweepResult :type Hit%20Result%20Structure%20%28by%20ref%29))
  (bind _asbp_finger (Utilities|Casting|CastToBP_Finger OtherActor))
  (CameraShakes|StartCameraShake (Game|GetPlayerCameraManager 0) "/Game/hadasjk/Effect/BP_CameraShake.BP_CameraShake_C" 1.0 "CameraLocal" "0, 0, 0")
  (Components|Activation|Activate (Variables|Default|GetNS) false)
  (Components|Timeline|SetPlayRate (Variables|Default|GetMoveUp) (/ 1.0 (Variables|Default|GetMoveUpTime)))
  (bind _alpha (Timeline|MoveUp PlayFromStart)
    (:Update
      (Transformation|SetActorLocation (Math|Vector|Lerp(Vector) (Variables|Default|GetStartLocation) (Variables|Default|GetMidLocation) _alpha) false false))
    (:Finished
      (Utilities|FlowControl|Delay 5.0)
      (Components|Timeline|SetPlayRate (Variables|Default|GetMoveWall) (/ 1.0 (Variables|Default|GetMoveWallTime)))
      (bind _alpha_2 (Timeline|MoveWall PlayFromStart)
        (:Update
          (Transformation|SetActorLocation (Math|Vector|Lerp(Vector) (Variables|Default|GetMidLocation) (+ (Variables|Default|GetMidLocation) (Variables|Default|GetWallDistance)) _alpha_2) false false))
        (:Finished
          (Utilities|FlowControl|Delay (Variables|Default|GetSpawnCoolTime))
          (Transformation|SetActorLocation (Variables|Default|GetStartLocation) false false)
          (Components|Activation|Deactivate (Variables|Default|GetNS)))))))

(event EventBeginPlay
  (Variables|Default|SetStartLocation (Transformation|GetActorLocation)))

(fn ConstructionScript)