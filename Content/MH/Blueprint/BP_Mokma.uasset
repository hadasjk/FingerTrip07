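; BP_Mokma is a carousel that runs while a BP_Finger overlaps its sphere.
; Overlap events toggle an active flag; beginning spawns a 2D sound, or stops the stored one if still valid, and ending stops it.
; While active, Tick spins the base and bobs two horses in opposite directions from their starting heights, using a cosine of game time.
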(event OnComponentBeginOverlap(Sphere)
  (params (OverlappedComponent :type Primitive%20Component%20Object%20Reference) (OtherActor :type Actor%20Object%20Reference) (OtherComp :type Primitive%20Component%20Object%20Reference) (OtherBodyIndex :type Integer) (bFromSweep :type Boolean) (SweepResult :type Hit%20Result%20Structure%20%28by%20ref%29))
  (Utilities|Casting|CastToBP_Finger OtherActor)
  (Variables|Default|SetbIsActive true)
  (Utilities|IsValid (Variables|Default|GetCurrentSound)
    (:Is%20Valid
      (Audio|Components|Audio|Stop (Variables|Default|GetCurrentSound)))
    (:Is%20Not%20Valid
      (bind _returnvalue (Audio|SpawnSound2D (Variables|Default|GetSound) 1.0 1.0 0.0 0))
      (Variables|Default|SetCurrentSound _returnvalue))))

(event OnComponentEndOverlap(Sphere)
  (params (OverlappedComponent :type Primitive%20Component%20Object%20Reference) (OtherActor :type Actor%20Object%20Reference) (OtherComp :type Primitive%20Component%20Object%20Reference) (OtherBodyIndex :type Integer))
  (bind _currentsound (Variables|Default|GetCurrentSound))
  (Utilities|Casting|CastToBP_Finger OtherActor)
  (Variables|Default|SetbIsActive false)
  (Utilities|IsValid _currentsound
    (:Is%20Valid
      (Audio|Components|Audio|Stop _currentsound))))

(event EventTick
  (params (DeltaSeconds :type Float%20%28single-precision%29))
  (bind _returnvalue (Utilities|Time|GetGameTimeinSeconds))
  (bind _updownspeed (Variables|Default|GetUpDownSpeed))
  (bind _updownheight (Variables|Default|GetUpDownHeight))
  (bind _returnvalue_2 (* _returnvalue _updownspeed))
  (bind _returnvalue_3 (Math|Trig|Cos(Radians) _returnvalue_2))
  (bind _returnvalue_4 (* _returnvalue_3 -1.0))
  (bind _returnvalue_5 (+ _returnvalue_4 1.0))
  (bind _returnvalue_6 (/ _returnvalue_5 2.0))
  (bind _returnvalue_7 (* _returnvalue_6 _updownheight))
  (if (Variables|Default|GetbIsActive)
    (Transformation|AddLocalRotation (Variables|Default|GetRotateBase) (Math|Rotator|MakeRotator 0.0 0.0 (* DeltaSeconds (Variables|Default|GetRotationSpeed))) false false)
    (Transformation|SetRelativeLocation (Variables|Default|GetHorse1) (Math|Vector|MakeVector 0.0 0.0 (+ _returnvalue_7 (Variables|Default|GetHorse1_StartZ))) false false)
    (Transformation|SetRelativeLocation (Variables|Default|GetHorse2) (Math|Vector|MakeVector 0.0 0.0 (+ (* _returnvalue_7 -1.0) (Variables|Default|GetHorse2_StartZ))) false false)))

(event EventBeginPlay
  (Variables|Default|SetHorse1_StartZ (.z (Variables|/Script/Engine.SceneComponent|GetRelativeLocation (Variables|Default|GetHorse1))))
  (Variables|Default|SetHorse2_StartZ (.z (Variables|/Script/Engine.SceneComponent|GetRelativeLocation (Variables|Default|GetHorse2)))))

(fn ConstructionScript)